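; Spawner actor that repeatedly creates random enemies from a list near itself, at a rate that rises as play time passes.
; Tick drives a DoOnce-gated spawn with random X offset, a height boost tied to list index 1, and a default AI controller.
; A random delay divided by TimeFromStart reopens the gate.
; A one-minute timer, re-armed from Tick, increments that counter to shorten the delay.
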(event `self.ReceiveBeginPlay`)

(event `self.ReceiveTick`
  (params (DeltaSeconds :type "Float (single-precision)"))
  (`self.Spawning`)
  (`self.SpawningReset`)
  (if (== (`KismetSystemLibrary.K2_GetTimerRemainingTimeHandle` (`self.timeToSpawn`)) 0.0)
    (bind _returnvalue (`KismetSystemLibrary.K2_SetTimerDelegate` (delegate `TimeCounter`) 60.0))
    (set `self.timeToSpawn` _returnvalue)))

(event `TimeCounter`
  (set `self.timeFromStart` (+ (`self.timeFromStart`) 1.0))
  (`KismetSystemLibrary.K2_ClearAndInvalidateTimerHandle` (`self.timeToSpawn`)))

(event `Spawning`
  (bind (_returnvalue_x _returnvalue_y _returnvalue_z) (`KismetMathLibrary.BreakVector` (`self.K2_GetActorLocation`)))
  (bind (_outitem _outindex) (`KismetArrayLibrary.Array_Random` (`self.enemyToSpawn`)))
  (`/Engine/EditorBlueprintResources/StandardMacros.DoOnce` false :!label _label
    (:`Completed`
      (bind _returnvalue (`|SpawnActorFromClass` _outitem (`KismetMathLibrary.MakeTransform` (`KismetMathLibrary.MakeVector` (+ _returnvalue_x (`KismetMathLibrary.RandomFloatInRange` -200.0 200.0)) 0.0 (+ _returnvalue_z (select `bool` (== _outindex 1) :`true` 400.0)))) "AdjustIfPossibleButDontSpawnIfColliding" "MultiplyWithRoot" null null))
      (`Pawn.SpawnDefaultController` _returnvalue))))

(event `SpawningReset`
  (`KismetSystemLibrary.Delay` (/ (`KismetMathLibrary.RandomFloatInRange` 10.0 15.0) (`self.timeFromStart`)))
  (goto _label :!via `Reset`))

(fn `UserConstructionScript`)