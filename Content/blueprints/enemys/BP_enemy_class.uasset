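; Base Paper2D enemy class that takes damage, plays hit and death flipbooks, and awards score to the player when killed.
; Damaged subtracts health and either plays a non-looping hurt flipbook or calls Dead, which adds PointsForKill to BP_player's score.
; A busy flag is set during these animations; when the flipbook finishes, Unbussy destroys a dead enemy or restores looping playback.
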(event `self.ReceiveTick`
  (params (DeltaSeconds :type "Float (single-precision)")))

(event `self.Sprite.OnFinishedPlaying`
  (`self.Unbussy`))

(fn `Damaged`
  (params (damageValue :type Integer))
  (bind _sprite (`self.Sprite`))
  (bind _output_get (set `self.health` (- (`self.health`) damageValue)))
  (if (< _output_get 1)
    (`self.Dead`)
    (else
      (set `self.Is Bussy` true)
      (`PaperFlipbookComponent.SetLooping` _sprite false)
      (`PaperFlipbookComponent.SetFlipbook` _sprite (`self.damagedFB`)))))

(fn `Dead`
  (bind _sprite (`self.Sprite`))
  (set `self.Is Bussy` true)
  (`PaperFlipbookComponent.SetLooping` _sprite false)
  (`PaperFlipbookComponent.SetFlipbook` _sprite (`self.deadFB`))
  (set `self.isDead` true)
  (bind _asbp_player (cast `/Game/blueprints/player/BP_player` (`GameplayStatics.GetPlayerPawn` 0)))
  (set `/Game/blueprints/player/BP_player.score` (+ (`/Game/blueprints/player/BP_player.score` _asbp_player) (`self.pointsForKill`)) _asbp_player))

(fn `Unbussy`
  (bind _sprite (`self.Sprite`))
  (if (`self.isDead`)
    (`self.K2_DestroyActor`)
    (else
      (set `self.Is Bussy` false)
      (`PaperFlipbookComponent.SetLooping` _sprite true)
      (`PaperFlipbookComponent.Play` _sprite))))

(fn `UserConstructionScript`)