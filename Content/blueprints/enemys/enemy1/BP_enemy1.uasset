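; BP_enemy1 is a flipbook-animated 2D enemy that chases the player and shoots fireballs, setting health, damage/death flipbooks and kill points for its parent class.
; Each Tick it picks idle or run animation, aims its SpringArm, faces the player and approaches until within horizontal range.
; When the player is close, Shoot spawns BP_enemy1_fireball at the Gun, then a re-armed one-second timer counts down the cooldown.
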(event `self.ReceiveBeginPlay`
  (`parent.ReceiveBeginPlay`)
  (set `self.health` 2)
  (set `self.damagedFB` "/Game/PaperModels/Enemy1/flipbooks/FB_enemy1_damage.FB_enemy1_damage")
  (set `self.deadFB` "/Game/PaperModels/Enemy1/flipbooks/FB_enemy1_dead.FB_enemy1_dead")
  (set `self.pointsForKill` 100))

(event `self.ReceiveTick`
  (params (DeltaSeconds :type "Float (single-precision)"))
  (`parent.ReceiveTick` DeltaSeconds)
  (`self.AnimUpdate`)
  (`self.Aim`)
  (`self.TurnFaceToPlayer`)
  (`self.MoveToPlayer`)
  (`self.ToShootCheck`))

(event `Shoot`
  (bind _sprite (`self.Sprite`))
  (if (and (`self.isReadyToShoot`) (not (`self.Is Bussy`)))
    (set `self.isReadyToShoot` false)
    (set `self.timeToShoot` (`self.shootRate`))
    (set `self.Is Shooting` true)
    (`PaperFlipbookComponent.SetLooping` _sprite false)
    (`PaperFlipbookComponent.SetFlipbook` _sprite "/Game/PaperModels/Enemy1/flipbooks/FB_enemy1_shoot.FB_enemy1_shoot")
    (`|SpawnActorFromClass` "/Game/blueprints/enemys/enemy1/BP_enemy1_fireball.BP_enemy1_fireball_C" (`SceneComponent.K2_GetComponentToWorld` (`self.gun`)) "Undefined" "MultiplyWithRoot" null null)))

(event `self.Sprite.OnFinishedPlaying`
  (set `self.Is Shooting` false))

(fn `Aim`
  (bind (_returnvalue_x _returnvalue_y _returnvalue_z) (`KismetMathLibrary.BreakVector` (`self.K2_GetActorLocation`)))
  (bind (_returnvalue_x_2 _returnvalue_y_2 _returnvalue_z_2) (`KismetMathLibrary.BreakVector` (`self.K2_GetActorLocation` (`GameplayStatics.GetPlayerPawn` 0))))
  (bind (_returnvalue_roll _returnvalue_pitch _returnvalue_yaw) (`KismetMathLibrary.BreakRotator` (`KismetMathLibrary.FindLookAtRotation` (`KismetMathLibrary.MakeVector` _returnvalue_x 0.0 _returnvalue_z) (`KismetMathLibrary.MakeVector` _returnvalue_x_2 0.0 _returnvalue_z_2))))
  (`SceneComponent.K2_SetWorldRotation` (`self.SpringArm`) (`KismetMathLibrary.MakeRotator` 0.0 _returnvalue_pitch _returnvalue_yaw) false false))

(fn `AnimUpdate`
  (bind _sprite (`self.Sprite`))
  (if (`self.Is Bussy`)
    _
    (elif (> (`KismetMathLibrary.VSize` (`self.GetVelocity`)) 0.0)
      (`PaperFlipbookComponent.SetFlipbook` _sprite "/Game/PaperModels/Enemy1/flipbooks/FB_enemy1_run.FB_enemy1_run")
      (else
        (`PaperFlipbookComponent.SetFlipbook` _sprite "/Game/PaperModels/Enemy1/flipbooks/FB_enemy1_idle.FB_enemy1_idle")))))

(fn `MoveToPlayer`
  (bind _returnvalue_x (`KismetMathLibrary.BreakVector` (`self.K2_GetActorLocation`)))
  (bind _returnvalue_x_2 (`KismetMathLibrary.BreakVector` (`self.K2_GetActorLocation` (`GameplayStatics.GetPlayerPawn` 0))))
  (if (> (`KismetMathLibrary.Vector_Distance` (`KismetMathLibrary.MakeVector` _returnvalue_x) (`KismetMathLibrary.MakeVector` _returnvalue_x_2)) 450.0)
    (`self.AddMovementInput` (`self.GetActorForwardVector`) 0.5)))

(fn `TimeToShootCountdown`
  (set `self.timeToShoot` (- (`self.timeToShoot`) 1))
  (`KismetSystemLibrary.K2_ClearAndInvalidateTimerHandle` (`self.timerToReadyShoot`)))

(fn `ToShootCheck`
  (if (`self.isReadyToShoot`)
    (if (< (`self.GetDistanceTo` (`GameplayStatics.GetPlayerPawn` 0)) 800.0)
      (`self.Shoot`))
    (elif (> (`self.timeToShoot`) 0)
      (if (== (`KismetSystemLibrary.K2_GetTimerRemainingTimeHandle` (`self.timerToReadyShoot`)) 0.0)
        (bind _returnvalue (`KismetSystemLibrary.K2_SetTimer` null "TimeToShootCountdown" 1.0))
        (set `self.timerToReadyShoot` _returnvalue)
        (else
          (set `self.isReadyToShoot` false)))
      (else
        (set `self.isReadyToShoot` true)))))

(fn `TurnFaceToPlayer`
  (bind _returnvalue_x (`KismetMathLibrary.BreakVector` (`self.K2_GetActorLocation`)))
  (bind _returnvalue_x_2 (`KismetMathLibrary.BreakVector` (`self.K2_GetActorLocation` (`GameplayStatics.GetPlayerPawn` 0))))
  (if (> _returnvalue_x _returnvalue_x_2)
    (`self.K2_SetActorRotation` (`KismetMathLibrary.MakeRotator` 0.0 0.0 180.0))
    (else
      (`self.K2_SetActorRotation` (`KismetMathLibrary.MakeRotator` 0.0)))))

(fn `UserConstructionScript`
  (`parent.UserConstructionScript`))