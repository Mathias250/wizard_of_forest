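; BP_enemy2 is a one-health flying flipbook enemy that homes in on the player and dies on contact.
; It disables character movement and uses projectile movement homed on the player's capsule, leaving MoveToPlayer uncalled.
; Tick updates the fly flipbook and yaws the enemy to face the player along X.
; Capsule overlap with the player calls Dead, while the DoOnce branch that would damage the player is unconnected.
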(event `self.ReceiveBeginPlay`
  (`parent.ReceiveBeginPlay`)
  (set `self.health` 1)
  (set `self.damagedFB` "/Game/PaperModels/Enemy2/flipbooks/FB_enemy2_dead.FB_enemy2_dead")
  (set `self.deadFB` "/Game/PaperModels/Enemy2/flipbooks/FB_enemy2_dead.FB_enemy2_dead")
  (set `self.pointsForKill` 50)
  (`ActorComponent.SetActive` (`self.CharacterMovement`) false false)
  (set `ProjectileMovementComponent.HomingTargetComponent` (`self.GetComponentByClass` (`GameplayStatics.GetPlayerPawn` 0) "/Script/Engine.CapsuleComponent") (`self.ProjectileMovement`)))

(event `self.ReceiveActorBeginOverlap`
  (params (OtherActor :type "Actor Object Reference"))
  (`parent.ReceiveActorBeginOverlap` OtherActor))

(event `self.ReceiveTick`
  (params (DeltaSeconds :type "Float (single-precision)"))
  (`parent.ReceiveTick` DeltaSeconds)
  (`self.AnimUptdate`)
  (`self.TurnFaceToPlayer`))

(event `self.CapsuleComponent.OnComponentBeginOverlap`
  (params (OverlappedComponent :type "PrimitiveComponent Object Reference") (OtherActor :type "Actor Object Reference") (OtherComp :type "PrimitiveComponent Object Reference") (OtherBodyIndex :type Integer) (bFromSweep :type Boolean) (SweepResult :type "HitResult Structure (by ref)"))
  (for _array_element (`self.GetOverlappingActors` "/Game/blueprints/player/BP_player.BP_player_C")
    (if (== _array_element (`GameplayStatics.GetPlayerPawn` 0))
      (set `self.health` 0)
      (`self.Dead`))))

(fn `AnimUptdate`
  (if (not (`self.Is Bussy`))
    (`PaperFlipbookComponent.SetFlipbook` (`self.Sprite`) "/Game/PaperModels/Enemy2/flipbooks/FB_enemy2_fly.FB_enemy2_fly")))

(fn `MoveToPlayer`
  (bind (_returnvalue_x _returnvalue_y _returnvalue_z) (`KismetMathLibrary.BreakVector` (`self.K2_GetActorLocation`)))
  (bind (_returnvalue_x_2 _returnvalue_y_2 _returnvalue_z_2) (`KismetMathLibrary.BreakVector` (`self.K2_GetActorLocation` (`GameplayStatics.GetPlayerPawn` 0))))
  (`self.AddMovementInput` (`KismetMathLibrary.GetDirectionUnitVector` (`KismetMathLibrary.MakeVector` _returnvalue_x 0.0 _returnvalue_z) (`KismetMathLibrary.MakeVector` _returnvalue_x_2 0.0 _returnvalue_z_2)) 0.3))

(fn `TurnFaceToPlayer`
  (bind _returnvalue_x (`KismetMathLibrary.BreakVector` (`self.K2_GetActorLocation`)))
  (bind _returnvalue_x_2 (`KismetMathLibrary.BreakVector` (`self.K2_GetActorLocation` (`GameplayStatics.GetPlayerPawn` 0))))
  (if (> _returnvalue_x _returnvalue_x_2)
    (`self.K2_SetActorRotation` (`KismetMathLibrary.MakeRotator` 0.0 0.0 180.0))
    (else
      (`self.K2_SetActorRotation` (`KismetMathLibrary.MakeRotator` 0.0)))))

(fn `UserConstructionScript`
  (`parent.UserConstructionScript`))