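; Player fireball projectile that damages enemies and can be hit back out after it returns to the player.
; Tick polls overlapping enemies, and a DoOnce limits each flight to one hit, which plays the end flipbook.
; When that animation finishes, TurnBack makes the fireball hittable and homes it onto the player's capsule.
; HittedBack relaunches it along the player's tagged shootDirection component and re-arms the damage gate.
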(event `self.ReceiveBeginPlay`
  (`parent.ReceiveBeginPlay`)
  (set `self.IsHittable` false))

(event `HitBackReset`
  (bind _paperflipbook (`self.PaperFlipbook`))
  (goto _label :!via `Reset`))

(event `self.ReceiveTick`
  (params (DeltaSeconds :type "Float (single-precision)"))
  (bind _paperflipbook (`self.PaperFlipbook`))
  (`parent.ReceiveTick` DeltaSeconds)
  (for _array_element (`self.GetOverlappingActors` "/Game/blueprints/enemys/BP_enemy_class.BP_enemy_class_C")
    (bind _asbp_enemy_class (cast `/Game/blueprints/enemys/BP_enemy_class` _array_element))
    (`/Engine/EditorBlueprintResources/StandardMacros.DoOnce` false :!label _label
      (:`Completed`
        (`/Game/blueprints/enemys/BP_enemy_class.Damaged` _asbp_enemy_class (`self.damageValue`))
        (`PaperFlipbookComponent.SetLooping` _paperflipbook false)
        (`PaperFlipbookComponent.SetFlipbook` _paperflipbook "/Game/PaperModels/PCharacter/flipbooks/FB_player_fireball_end.FB_player_fireball_end")
        (set `self.hitted` true)))))

(event `self.PaperFlipbook.OnFinishedPlaying`
  (bind _paperflipbook (`self.PaperFlipbook`))
  (`PaperFlipbookComponent.SetLooping` _paperflipbook true)
  (`PaperFlipbookComponent.Play` _paperflipbook)
  (if (`self.hitted`)
    (`self.TurnBack`)))

(fn `HittedBack`
  (bind _projectilemovement (`self.ProjectileMovement`))
  (bind _speed (`self.speed`))
  (`PaperFlipbookComponent.SetFlipbook` (`self.PaperFlipbook`) "/Game/PaperModels/PCharacter/flipbooks/FB_player_fireball.FB_player_fireball")
  (set `self.IsHittable` false)
  (for _array_element (`self.GetComponentsByTag` (`GameplayStatics.GetPlayerPawn` 0) "/Script/Engine.CapsuleComponent" "shootDirection")
    (set `self.playerShootDirection` (`SceneComponent.K2_GetComponentRotation` _array_element)))
  (set `MovementComponent.Velocity` (* (`KismetMathLibrary.GetForwardVector` (`self.playerShootDirection`)) (`self.speed`)) _projectilemovement)
  (set `ProjectileMovementComponent.bIsHomingProjectile` false _projectilemovement)
  (set `ProjectileMovementComponent.MaxSpeed` _speed _projectilemovement)
  (set `ProjectileMovementComponent.InitialSpeed` _speed _projectilemovement)
  (`self.HitBackReset`)
  (set `self.hitted` false))

(fn `TurnBack`
  (bind _projectilemovement (`self.ProjectileMovement`))
  (`PaperFlipbookComponent.SetFlipbook` (`self.PaperFlipbook`) "/Game/PaperModels/PCharacter/flipbooks/FB_player_fireball_back.FB_player_fireball_back")
  (set `self.IsHittable` true)
  (set `MovementComponent.Velocity` (0.0 0.0 0.0) _projectilemovement)
  (set `ProjectileMovementComponent.bIsHomingProjectile` true _projectilemovement)
  (set `ProjectileMovementComponent.HomingAccelerationMagnitude` 1000.0 _projectilemovement)
  (set `ProjectileMovementComponent.MaxSpeed` 500.0 _projectilemovement)
  (set `ProjectileMovementComponent.InitialSpeed` 500.0 _projectilemovement)
  (set `ProjectileMovementComponent.HomingTargetComponent` (`self.GetComponentByClass` (`GameplayStatics.GetPlayerPawn` 0) "/Script/Engine.CapsuleComponent") _projectilemovement))

(fn `UserConstructionScript`
  (`parent.UserConstructionScript`))